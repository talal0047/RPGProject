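; Actor component that tracks health and stamina for BP_ThirdPersonCharacter, caching the cast owner on BeginPlay.
; Functions lower, raise or extend the maximum of each stat, then push the current/max ratio to the owner's HUD progress bars.
; Both Decrease functions return whether health is depleted, including the stamina one.
; Increases clamp to maximum, though the health clamp tests CurrentStamina against MaxHealth; decreases are unclamped.
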(event `self.ReceiveBeginPlay`
  (bind _asbp_third_person_character (cast `/Game/ThirdPerson/Blueprints/BP_ThirdPersonCharacter` (`self.GetOwner`)))
  (set `self.BP Third Person Character` _asbp_third_person_character))

(fn `Decrease Health`
  (params (Damage :type "Float (double-precision)"))
  (returns (`Is Player Dead?` :type Boolean))
  (bind _output_get (set `self.Current Health` (- (`self.Current Health`) Damage)))
  (`ProgressBar.SetPercent` (`/Game/UI/WB_MainHUD.HealthBar` (`/Game/ThirdPerson/Blueprints/BP_ThirdPersonCharacter.HUD  Widget` (`self.BP Third Person Character`))) (/ _output_get (`self.Max Health`)))
  (if (<= (`self.Current Health`) 0.0)
    (return true)
    (else
      (return false))))

(fn `Decrease Stamina`
  (params (`Depleated Stamina` :type "Float (double-precision)"))
  (returns (`Not Stamina Left` :type Boolean))
  (bind _output_get (set `self.Current Stamina` (- (`self.Current Stamina`) `Depleated Stamina`)))
  (`ProgressBar.SetPercent` (`/Game/UI/WB_MainHUD.StaminaBar` (`/Game/ThirdPerson/Blueprints/BP_ThirdPersonCharacter.HUD  Widget` (`self.BP Third Person Character`))) (/ _output_get (`self.Max Stamina`)))
  (if (<= (`self.Current Health`) 0.0)
    (return true)
    (else
      (return false))))

(fn `Increase Health`
  (params (`Increment Health` :type "Float (double-precision)"))
  (set `self.Current Health` (+ (`self.Current Health`) `Increment Health`))
  (if (> (`self.Current Stamina`) (`self.Max Health`))
    (set `self.Current Health` (`self.Max Health`)))
  (`ProgressBar.SetPercent` (`/Game/UI/WB_MainHUD.HealthBar` (`/Game/ThirdPerson/Blueprints/BP_ThirdPersonCharacter.HUD  Widget` (`self.BP Third Person Character`))) (/ (`self.Current Health`) (`self.Max Health`))))

(fn `Increase Max Health`
  (params (`Health Increamentation` :type "Float (double-precision)"))
  (set `self.Max Health` (+ (`self.Max Health`) `Health Increamentation`))
  (`ProgressBar.SetPercent` (`/Game/UI/WB_MainHUD.HealthBar` (`/Game/ThirdPerson/Blueprints/BP_ThirdPersonCharacter.HUD  Widget` (`self.BP Third Person Character`))) (/ (`self.Current Health`) (`self.Max Health`))))

(fn `Increase Max Stamina`
  (params (`Increase Stamina` :type "Float (double-precision)"))
  (set `self.Max Stamina` (+ (`self.Max Stamina`) `Increase Stamina`))
  (`ProgressBar.SetPercent` (`/Game/UI/WB_MainHUD.StaminaBar` (`/Game/ThirdPerson/Blueprints/BP_ThirdPersonCharacter.HUD  Widget` (`self.BP Third Person Character`))) (/ (`self.Current Stamina`) (`self.Max Stamina`))))

(fn `Increase Stamina`
  (params (`Increase Stamina` :type "Float (double-precision)"))
  (bind _output_get (set `self.Current Stamina` (+ (`self.Current Stamina`) `Increase Stamina`)))
  (if (> _output_get (`self.Max Stamina`))
    (set `self.Current Stamina` (`self.Max Stamina`)))
  (`ProgressBar.SetPercent` (`/Game/UI/WB_MainHUD.StaminaBar` (`/Game/ThirdPerson/Blueprints/BP_ThirdPersonCharacter.HUD  Widget` (`self.BP Third Person Character`))) (/ (`self.Current Stamina`) (`self.Max Stamina`))))