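; Actor component that runs a four-step sword combo, including a kick, on the owning BP_ThirdPersonCharacter.
; IA_Attack starts the attack selected by AttachIndex when CanAttack is set, or buffers it in SaveAttack during an attack.
; Each step plays a montage behind a DoOnce and short delay, then advances the index.
; SwordAttackCombo, not called within this graph, consumes buffered input to continue or resets the combo.
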(event `self.ReceiveBeginPlay`
  (bind _asbp_third_person_character (cast `/Game/ThirdPerson/Blueprints/BP_ThirdPersonCharacter` (`self.GetOwner`)))
  (set `self.Character Mesh` (`Character.Mesh` _asbp_third_person_character)))

(event `Attack 1`
  ;[0.05098 0.05098 0.05098] Attack 1
  (`/Engine/EditorBlueprintResources/StandardMacros.DoOnce` false :!label _label
    (:`Completed`
      (`KismetSystemLibrary.Delay` 0.1)
      (`|PlayMontage` (`self.Character Mesh`) "/Game/Characters/RPG_Character/Animation/SwordAttacks/Attack1_Montage.Attack1_Montage"
        (:`then`
          (set `self.attachIndex` 1)
          (goto _label :!via `Reset`))))))

(event `EnhancedInput|/Game/ThirdPerson/Input/Actions/IA_Attack`
  (params (ActionValue :type Boolean) (ElapsedSeconds :type "Float (double-precision)") (TriggeredSeconds :type "Float (double-precision)") (InputAction :type "InputAction Object Reference" :default "/Game/ThirdPerson/Input/Actions/IA_Attack.IA_Attack"))
  ;[0.05098 0.05098 0.05098] Attack Input
  (:`Started`
    (if (`self.canAttack?`)
      (`self.SwordAttack`))))

(event `Attack 2`
  ;[0.05098 0.05098 0.05098] Attack 2
  (`/Engine/EditorBlueprintResources/StandardMacros.DoOnce` false :!label _label_2
    (:`Completed`
      (`KismetSystemLibrary.Delay` 0.1)
      (`|PlayMontage` (`self.Character Mesh`) "/Game/Characters/RPG_Character/Animation/SwordAttacks/Attack2_Montage.Attack2_Montage"
        (:`then`
          (set `self.attachIndex` 2)
          (goto _label_2 :!via `Reset`))))))

(event `SwordAttack`
  ;[0.05098 0.05098 0.05098] Sword Attack
  (if (`self.isAttacking?`)
    (set `self.saveAttack?` true)
    (else
      (set `self.isAttacking?` true)
      (switch `int` (`self.attachIndex`) :!label _label_3
        (:`0`
          (`self.Attack 1`))
        (:`1`
          (`self.Attack 2`))
        (:`2`
          (`self.Attack 3`))
        (:`3`
          (`self.Attack 4`))))))

(event `SwordAttackCombo`
  ;[0.05098 0.05098 0.05098] Combo  Continue
  (if (`self.saveAttack?`)
    (set `self.saveAttack?` false)
    (goto _label_3)
    (else
      (`self.StopCombo`))))

(event `Attack 3`
  ;[0.05098 0.05098 0.05098] Attack 3
  (`/Engine/EditorBlueprintResources/StandardMacros.DoOnce` false :!label _label_4
    (:`Completed`
      (`KismetSystemLibrary.Delay` 0.1)
      (`|PlayMontage` (`self.Character Mesh`) "/Game/Characters/RPG_Character/Animation/SwordAttacks/Kick_Montage.Kick_Montage"
        (:`then`
          (set `self.attachIndex` 3)
          (goto _label_4 :!via `Reset`))))))

(event `StopCombo`
  ;[0.05098 0.05098 0.05098] Stop Combo
  (set `self.isAttacking?` false)
  (set `self.attachIndex` 0))

(event `Attack 4`
  ;[0.05098 0.05098 0.05098] Attack 4
  (`/Engine/EditorBlueprintResources/StandardMacros.DoOnce` false :!label _label_5
    (:`Completed`
      (`KismetSystemLibrary.Delay` 0.1)
      (`|PlayMontage` (`self.Character Mesh`) "/Game/Characters/RPG_Character/Animation/SwordAttacks/Attack3_Montage.Attack3_Montage"
        (:`then`
          (set `self.attachIndex` 4)
          (goto _label_5 :!via `Reset`))))))